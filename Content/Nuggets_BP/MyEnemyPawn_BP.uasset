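; Enemy pawn Blueprint that shows a screen-space target rectangle over itself, with distance and lock-on state.
; BeginPlay creates a fixed-size, center-aligned TargetRect widget and adds it to the viewport; Destroyed removes it.
; Each Tick projects the actor's location to screen to position the widget, then feeds it the player distance in whole meters and the GetLockOnStatus result.
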(event EventBeginPlay
  (bind _returnvalue (UserInterface|CreateWidget "/Game/Nuggets_BP/TargetRect.TargetRect_C"))
  (bind _output_get (Variables|Default|SetTargetRect _returnvalue))
  (Class|UserWidget|SetDesiredSizeinViewport _output_get "(X=200.000000,Y=200.000000)")
  (Class|UserWidget|SetAlignmentinViewport _output_get "(X=0.500000,Y=0.500000)")
  (UserInterface|Viewport|AddtoViewport _returnvalue 0))

(event Collision|EventActorBeginOverlap
  (params (OtherActor :type Actor%20Object%20Reference)))

(event EventTick
  (params (DeltaSeconds :type Float%20%28single-precision%29))
  (bind _targetrect (Variables|Default|GetTargetRect))
  (Variables|/Game/Nuggets_BP/TargetRect.TargetRect_C|SetTargetDistance _targetrect (Math|Float|Truncate (/ (Transformation|GetDistanceTo (Game|Player|GetPlayerPawn 0)) 1e+02)))
  (Class|UserWidget|SetPositioninViewport _targetrect (.ScreenPosition (Class|GameplayStatics|ProjectWorldtoScreen (Game|GetPlayerController 0) (Transformation|GetActorLocation) false)) true)
  (bind _returnvalue (Class|EnemyPawn|GetLockonStatus))
  (Variables|/Game/Nuggets_BP/TargetRect.TargetRect_C|SetLockOnStatus (Variables|Default|GetTargetRect) _returnvalue))

(event EventDestroyed
  (Widget|RemovefromParent (Variables|Default|GetTargetRect)))

(fn ConstructionScript)