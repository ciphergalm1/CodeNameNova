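; Spawn volume that periodically adds alerted enemy pawns to the level while the enemy count is low.
; On BeginPlay it caches the Nova game state and starts a looping timer with a randomized interval, chosen once.
; Each tick of that timer checks the game state's enemy count, then spawns a batch at random points in the volume, sets their alert status and raises the clamped count.
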(event EventBeginPlay
  (bind _asnova_game_state_base (Utilities|Casting|CastToNovaGameStateBase (Game|GetGameState)))
  (Variables|Default|SetcurrentGameState _asnova_game_state_base)
  (Utilities|Time|SetTimerbyFunctionName 0 "DelayedSpawn" (Math|Random|RandomFloatinRange 3e+01 6e+01) true))

(event Collision|EventActorBeginOverlap
  (params (OtherActor :type Actor%20Object%20Reference)))

(event EventTick
  (params (DeltaSeconds :type Float%20%28single-precision%29)))

(fn ConstructionScript)

(fn DelayedSpawn
  (bind _currentgamestate (Variables|Default|GetcurrentGameState))
  (if (<= (Variables|/Game/Nuggets_BP/NovaGameStateBase.NovaGameStateBase_C|GetEnemyInLevel (Variables|Default|GetcurrentGameState)) 8)
    (Utilities|FlowControl|ForLoopwithBreak 0 3
      (:LoopBody
        (bind _returnvalue (Game|SpawnActorfromClass "/Game/Nuggets_BP/MyEnemyPawn_BP.MyEnemyPawn_BP_C" (Math|Transform|MakeTransform (Class|SpawnVolume|GetRandomPoint) (Transformation|GetActorRotation)) "AlwaysSpawn" 0 0))
        (Class|EnemyPawn|SetAlertStatus _returnvalue 1)
        (bind _result (Math|Integer|IncrementInt (Variables|/Game/Nuggets_BP/NovaGameStateBase.NovaGameStateBase_C|GetEnemyInLevel _currentgamestate))
          (:%20%20
            (Variables|/Game/Nuggets_BP/NovaGameStateBase.NovaGameStateBase_C|SetEnemyInLevel _currentgamestate (Math|Integer|Clamp(Integer) _result 0 12))))))))