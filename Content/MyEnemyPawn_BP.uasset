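; Enemy pawn Blueprint that shows a TargetRect widget on screen over its own position.
; It creates the widget and adds it to the viewport on BeginPlay, then removes it when the pawn is destroyed.
; Each Tick projects the actor's world location to screen space for the first player controller and moves the widget there, correcting for DPI scale.
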(event EventBeginPlay
  (bind _returnvalue (UserInterface|CreateWidget "/Game/Nuggets_BP/TargetRect.TargetRect_C"))
  (bind _output_get (Variables|Default|SetTargetRect _returnvalue))
  (UserInterface|Viewport|AddtoViewport _returnvalue 0))

(event Collision|EventActorBeginOverlap
  (params (OtherActor :type Actor%20Object%20Reference)))

(event EventTick
  (params (DeltaSeconds :type Float%20%28single-precision%29))
  (Class|UserWidget|SetPositioninViewport (Variables|Default|GetTargetRect) (.ScreenPosition (Class|GameplayStatics|ProjectWorldtoScreen (Game|GetPlayerController 0) (Transformation|GetActorLocation) false)) true))

(event EventDestroyed
  (Widget|RemovefromParent (Variables|Default|GetTargetRect)))

(fn ConstructionScript)